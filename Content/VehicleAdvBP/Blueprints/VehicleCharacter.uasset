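; Player-driven four-wheeled vehicle Blueprint that turns input into driving controls and drives its engine audio.
; MoveForward and MoveRight axes feed throttle and steering on the WheeledVehicleMovementComponent4W, and the Handbrake action engages the brake while held.
; Each Tick passes absolute forward speed to the audio component's RPM parameter, using road speed as a stand-in for engine revs.
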(event `InputAxis|MoveForward`
  (params (AxisValue :type "Float (single-precision)"))
  ;[1 1 1] Movement control
  (`WheeledVehicleMovementComponent.SetThrottleInput` (`self.WheeledVehicleMovementComponent4W`) AxisValue))

(event `InputAxis|MoveRight`
  (params (AxisValue :type "Float (single-precision)"))
  ;[1 1 1] Movement control
  (`WheeledVehicleMovementComponent.SetSteeringInput` (`self.WheeledVehicleMovementComponent4W`) AxisValue))

(event `InputAction|Handbrake`
  (params (Key :type "Key Structure" :default "AnyKey"))
  (bind _wheeledvehiclemovementcomponent4w (`self.WheeledVehicleMovementComponent4W`))
  ;[1 1 1] Movement control
  (:`Pressed`
    (`WheeledVehicleMovementComponent.SetHandbrakeInput` _wheeledvehiclemovementcomponent4w true))
  (:`Released`
    (`WheeledVehicleMovementComponent.SetHandbrakeInput` _wheeledvehiclemovementcomponent4w false)))

(event `self.ReceiveTick`
  (params (DeltaSeconds :type "Float (single-precision)"))
  ;[1 1 1] Audio
  (`AudioComponent.SetFloatParameter` (`self.Audio1`) "RPM" (`KismetMathLibrary.Abs` (`WheeledVehicleMovementComponent.GetForwardSpeed` (`self.WheeledVehicleMovementComponent4W`)))))

(fn `UserConstructionScript`)