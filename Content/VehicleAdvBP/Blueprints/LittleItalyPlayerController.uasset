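; Player controller for a timed taxi-style driving game, tracking countdown, score and completed tasks.
; Tick decrements RemainingTime about once per second.
; GenerateEvent spawns a passenger and StartEvent an end point from the VehicleBlueprint's point arrays, each setting TargetPosition through a separate random pick that can differ from the spawn.
; CompleteEvent awards points for time left within MaxEventTime, then generates the next passenger.
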(event `self.ReceiveTick`
  (params (DeltaSeconds :type "Float (single-precision)"))
  (bind _returnvalue (+ (`self.delta`) DeltaSeconds))
  (`/Engine/EditorBlueprintResources/StandardMacros.CompareFloat` _returnvalue 1.0
    (:`>`
      (set `self.delta` 0.0 :!label _label)
      (set `self.remainingTime` (- (`self.remainingTime`) 1)))
    (:`==`
      (goto _label))
    (:`<`
      (set `self.delta` _returnvalue))))

(fn `CompleteEvent`
  (bind _returnvalue (- (`self.maxEventTime`) (- (`self.startEventTime`) (`self.remainingTime`))))
  ;[1 1 1] points
  (`/Engine/EditorBlueprintResources/StandardMacros.CompareInt` _returnvalue
    (:`>`
      (set `self.Points` (+ (`self.Points`) (* _returnvalue 100))))
    (:`==`
      _)
    (:`<`
      _))
  ;[1 1 1] completed tasks
  (set `self.CompletedTasks` (+ (`self.CompletedTasks`) 1))
  (`self.GenerateEvent`))

(fn `GenerateEvent`
  (bind _asvehicle_blueprint (cast `/Game/VehicleAdvBP/Blueprints/VehicleBlueprint` (`GameplayStatics.GetPlayerPawn` 0)))
  (bind _startpoints (`/Game/VehicleAdvBP/Blueprints/VehicleBlueprint.StartPoints` _asvehicle_blueprint))
  (bind _returnvalue (`self.K2_GetActorLocation` (`KismetArrayLibrary.Array_Get` _startpoints (`KismetMathLibrary.RandomIntegerInRange` 0 (- (`KismetArrayLibrary.Array_Length` _startpoints) 1)))))
  (`|SpawnActorFromClass` "/Game/VehicleAdvBP/Blueprints/Passenger_BP.Passenger_BP_C" (`KismetMathLibrary.MakeTransform` _returnvalue) "Undefined" "OverrideRootScale")
  (set `self.TargetPosition` _returnvalue))

(fn `StartEvent`
  (bind _asvehicle_blueprint (cast `/Game/VehicleAdvBP/Blueprints/VehicleBlueprint` (`GameplayStatics.GetPlayerPawn` 0)))
  (set `self.startEventTime` (`self.remainingTime`))
  (bind _endpoints (`/Game/VehicleAdvBP/Blueprints/VehicleBlueprint.EndPoints` _asvehicle_blueprint))
  (bind _returnvalue (`self.K2_GetActorLocation` (`KismetArrayLibrary.Array_Get` _endpoints (`KismetMathLibrary.RandomIntegerInRange` 0 (- (`KismetArrayLibrary.Array_Length` _endpoints) 1)))))
  (`|SpawnActorFromClass` "/Game/VehicleAdvBP/Blueprints/EndPoint_BP.EndPoint_BP_C" (`KismetMathLibrary.MakeTransform` _returnvalue) "Undefined" "OverrideRootScale")
  (set `self.TargetPosition` _returnvalue))

(fn `UserConstructionScript`)