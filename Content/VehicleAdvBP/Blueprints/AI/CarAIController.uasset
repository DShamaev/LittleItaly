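; AI controller for city traffic cars that drives a random route through the behavior tree.
; On BeginPlay it picks four random StartPoints from the player's VehicleBlueprint, writes their locations to the blackboard as TargetPoint0–3, then runs CityTrafficBehaviour.
; RideToLocation looks unfinished: it computes a nav path but ignores it, applying fixed full throttle and steering to the controlled vehicle.
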(event `self.ReceiveBeginPlay`
  (bind _route (`self.Route`))
  (bind _asvehicle_blueprint (cast `/Game/VehicleAdvBP/Blueprints/VehicleBlueprint` (`self.K2_GetPawn` (`GameplayStatics.GetPlayerController` 0))))
  (for _ (range 4)
    (bind _startpoints (`/Game/VehicleAdvBP/Blueprints/VehicleBlueprint.StartPoints` _asvehicle_blueprint))
    (`KismetArrayLibrary.Array_Add` _route (`self.K2_GetActorLocation` (`KismetArrayLibrary.Array_Get` _startpoints (`KismetMathLibrary.RandomIntegerInRange` 0 (- (`KismetArrayLibrary.Array_Length` _startpoints) 1))))))
  (bind _blackboardcomponent (`self.UseBlackboard` "/Game/VehicleAdvBP/Blueprints/AI/CityTrafficBlackboard.CityTrafficBlackboard"))
  (for _index (range 4)
    (`BlackboardComponent.SetValueAsVector` _blackboardcomponent (`KismetStringLibrary.Conv_StringToName` (`KismetStringLibrary.Concat_StrStr` "TargetPoint" (`KismetStringLibrary.Conv_IntToString` _index))) (`KismetArrayLibrary.Array_Get` _route _index)))
  (`self.RunBehaviorTree` "/Game/VehicleAdvBP/Blueprints/AI/CityTrafficBehaviour.CityTrafficBehaviour"))

(fn `RideToLocation`
  (params (TargetPoint :type "Vector Structure"))
  (bind _returnvalue (`self.K2_GetPawn`))
  (bind _returnvalue_2 (`NavigationSystem.FindPathToLocationSynchronously` (`self.K2_GetActorLocation` _returnvalue) TargetPoint _returnvalue))
  (bind _asvehicle_blueprint (cast `/Game/VehicleAdvBP/Blueprints/VehicleBlueprint` _returnvalue))
  (bind _vehiclemovement (`WheeledVehicle.VehicleMovement` _asvehicle_blueprint))
  (`WheeledVehicleMovementComponent.SetThrottleInput` _vehiclemovement 1.0)
  (`WheeledVehicleMovementComponent.SetSteeringInput` _vehiclemovement 1.0))

(fn `UserConstructionScript`)